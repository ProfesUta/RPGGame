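; BP_Chest is a one-time openable chest that rewards the player with XP and an item.
; Its OpenChest function uses a flag to play the open animation only once, then casts player 0's character to BP_ThirdPersonCharacter.
; Through that character, it reports the chest to the quest component, adds XP via the player stats component and returns the Item to the caller.
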(fn `Open Chest`
  (returns (Item :type "/Game/Equipment_System/S_Slots Structure"))
  (if (not (`self.ChestOpened`))
    (set `self.ChestOpened` true)
    (`SkeletalMeshComponent.PlayAnimation` (`self.Chest`) "/Game/AllForMaps/Chest/Chest_Open.Chest_Open" false)
    (bind _asbp_third_person_character (cast `/Game/ThirdPerson/Blueprints/BP_ThirdPersonCharacter` (`GameplayStatics.GetPlayerCharacter` 0)))
    (`/Game/Quest_System/BPC_Quest.Open Chest` (`/Game/ThirdPerson/Blueprints/BP_ThirdPersonCharacter.BPC_Quest` _asbp_third_person_character) self)
    (`/Game/Blueprints/BPC_PlayerStats.Increase XP` (`/Game/ThirdPerson/Blueprints/BP_ThirdPersonCharacter.BPC_PlayerStats` _asbp_third_person_character) (`self.Added XP`))
    (return (`self.Item`))))

(fn `UserConstructionScript`)
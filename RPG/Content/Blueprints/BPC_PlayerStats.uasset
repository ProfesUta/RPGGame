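; Actor component that tracks health, stamina, XP and level for the player character, with health also supported on dummy and AI owners.
; BeginPlay waits a tick, detects the owner type by casting, and initializes its bars.
; DecreaseHealth updates the matching bar and reports depletion; other stat functions write directly to the player HUD.
; Reaching max XP levels up, resetting XP, raising the threshold, and playing sounds, animation and Niagara effect.
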(event `self.ReceiveBeginPlay`
  (`KismetSystemLibrary.DelayUntilNextTick`)
  (bind _asbp_third_person_character (cast `/Game/ThirdPerson/Blueprints/BP_ThirdPersonCharacter` (`self.GetOwner`))
    (:`then`
      (set `self.Player Character BP` _asbp_third_person_character)
      (set `self.IsPlayer` true)
      (`/Game/UI/WB_RoundStaminaBar.SetPercentage` (`/Game/UI/WB_HUD.WB_RoundStaminaBar` (`/Game/ThirdPerson/Blueprints/BP_ThirdPersonCharacter.HUD Widget` (`self.Player Character BP`))) (/ (`self.Current Stamina`) (`self.Max Stamina`)))
      (set `self.CharacterType` "NewEnumerator3"))
    (:`CastFailed`
      (bind _asbp_dummy (cast `/Game/Blueprints/BP_Dummy` (`self.GetOwner`))
        (:`then`
          (set `self.Dummy BP` _asbp_dummy)
          (set `self.IsPlayer` false)
          (set `self.CharacterType` "NewEnumerator1"))
        (:`CastFailed`
          (bind _asbp_ai (cast `/Game/AI/BP_AI` (`self.GetOwner`)))
          (set `self.AI BP` _asbp_ai)
          (set `self.IsPlayer` false)
          (set `self.CharacterType` "NewEnumerator2")))))
  (`/Game/UI/WB_RoundHPBar.SetPercent` (select `/Game/Blueprints/E_Character_Types` (`self.CharacterType`) :`NewEnumerator1` (`/Game/UI/WB_DummyHealth.WB_RoundHPBar` (`/Game/Blueprints/BP_Dummy.HealthBar UI` (`self.Dummy BP`))) :`NewEnumerator2` (`/Game/UI/WB_DummyHealth.WB_RoundHPBar` (`/Game/AI/BP_AI.HealthBar UI` (`self.AI BP`))) :`NewEnumerator3` (`/Game/UI/WB_HUD.WB_RoundHPBar` (`/Game/ThirdPerson/Blueprints/BP_ThirdPersonCharacter.HUD Widget` (`self.Player Character BP`)))) (/ (`self.Current Health`) (`self.Max Health`)))
  (if (`self.IsPlayer`)
    (`ProgressBar.SetPercent` (`/Game/UI/WB_HUD.XPBar` (`/Game/ThirdPerson/Blueprints/BP_ThirdPersonCharacter.HUD Widget` (`self.Player Character BP`))) (/ (`self.XP`) (`self.Max Xp`)))
    (`TextBlock.SetText` (`/Game/UI/WB_HUD.XPText` (`/Game/ThirdPerson/Blueprints/BP_ThirdPersonCharacter.HUD Widget` (`self.Player Character BP`))) (`|FormatText` "{Current XP} / {Max XP}" (`self.XP`) (`self.Max Xp`)))
    (`TextBlock.SetText` (`/Game/UI/WB_HUD.levelText` (`/Game/ThirdPerson/Blueprints/BP_ThirdPersonCharacter.HUD Widget` (`self.Player Character BP`))) (`KismetTextLibrary.Conv_IntToText` (`self.Level`)))))

(fn `Decrease Health`
  (params (Damage :type "Float (double-precision)"))
  (returns (`Is Player Dead?` :type Boolean))
  (if (not (<= (`self.Current Health`) 0.0))
    (bind _output_get (set `self.Current Health` (- (`self.Current Health`) Damage)))
    (`/Game/UI/WB_RoundHPBar.SetPercent` (select `/Game/Blueprints/E_Character_Types` (`self.CharacterType`) :`NewEnumerator1` (`/Game/UI/WB_DummyHealth.WB_RoundHPBar` (`/Game/Blueprints/BP_Dummy.HealthBar UI` (`self.Dummy BP`))) :`NewEnumerator2` (`/Game/UI/WB_DummyHealth.WB_RoundHPBar` (`/Game/AI/BP_AI.HealthBar UI` (`self.AI BP`))) :`NewEnumerator3` (`/Game/UI/WB_HUD.WB_RoundHPBar` (`/Game/ThirdPerson/Blueprints/BP_ThirdPersonCharacter.HUD Widget` (`self.Player Character BP`)))) (/ _output_get (`self.Max Health`)))
    (if (<= (`self.Current Health`) 0.0)
      _
      (else
        (return false))))
  (return true))

(fn `Decrease Stamina`
  (params (`Stamina Depleted` :type "Float (double-precision)"))
  (returns (`Not Stamina Left` :type Boolean))
  (if (not (<= (`self.Current Stamina`) 0.0))
    (set `self.Current Stamina` (- (`self.Current Stamina`) `Stamina Depleted`))
    (`/Game/UI/WB_RoundStaminaBar.SetPercentage` (`/Game/UI/WB_HUD.WB_RoundStaminaBar` (`/Game/ThirdPerson/Blueprints/BP_ThirdPersonCharacter.HUD Widget` (`self.Player Character BP`))) (/ (`self.Current Stamina`) (`self.Max Stamina`)))
    (if (<= (`self.Current Stamina`) 0.0)
      _
      (else
        (return false))))
  (return true))

(fn `Increase Health`
  (params (`Added Health` :type "Float (double-precision)"))
  (set `self.Current Health` (+ (`self.Current Health`) `Added Health`))
  (if (> (`self.Current Health`) (`self.Max Health`))
    (set `self.Current Health` (`self.Max Health`)))
  (`/Game/UI/WB_RoundHPBar.SetPercent` (`/Game/UI/WB_HUD.WB_RoundHPBar` (`/Game/ThirdPerson/Blueprints/BP_ThirdPersonCharacter.HUD Widget` (`self.Player Character BP`))) (/ (`self.Current Health`) (`self.Max Health`))))

(fn `Increase LVL`
  (params (`Added LVL` :type Integer))
  (bind _hud_widget (`/Game/ThirdPerson/Blueprints/BP_ThirdPersonCharacter.HUD Widget` (`self.Player Character BP`)))
  (set `self.Level` (+ (`self.Level`) `Added LVL`))
  (set `self.Max Xp` (+ (`self.Max Xp`) 150.0))
  (set `self.XP` 0.0)
  (`TextBlock.SetText` (`/Game/UI/WB_HUD.levelText` (`/Game/ThirdPerson/Blueprints/BP_ThirdPersonCharacter.HUD Widget` (`self.Player Character BP`))) (`KismetTextLibrary.Conv_IntToText` (`self.Level`)))
  (`GameplayStatics.PlaySound2D` "/Game/Audio/UI/LevelUp1.LevelUp1" 1.0 1.0 0.0 null null)
  (`GameplayStatics.PlaySound2D` "/Game/Audio/UI/LevelUp2.LevelUp2" 1.0 1.0 0.0 null null)
  (`/Game/UI/WB_HUD.Play Level Up Animation` _hud_widget)
  (`TextBlock.SetText` (`/Game/UI/WB_HUD.levelTextAnimation` _hud_widget) (`KismetTextLibrary.Conv_IntToText` (`self.Level`)))
  (`NiagaraFunctionLibrary.SpawnSystemAttached` "/Game/NS_LevelUp.NS_LevelUp" (`Character.Mesh` (`self.Player Character BP`)) "None" (0.0 0.0 0.0) (struct) "KeepRelativeOffset" true true "AutoRelease"))

(fn `Increase Max Health`
  (params (`Health Incremention` :type "Float (double-precision)"))
  (set `self.Max Health` (+ (`self.Max Health`) `Health Incremention`))
  (`/Game/UI/WB_RoundHPBar.SetPercent` (`/Game/UI/WB_HUD.WB_RoundHPBar` (`/Game/ThirdPerson/Blueprints/BP_ThirdPersonCharacter.HUD Widget` (`self.Player Character BP`))) (/ (`self.Current Health`) (`self.Max Health`))))

(fn `Increase Max Stamina`
  (params (`Added Stamina` :type "Float (double-precision)"))
  (set `self.Max Stamina` (+ (`self.Max Stamina`) `Added Stamina`))
  (`/Game/UI/WB_RoundStaminaBar.SetPercentage` (`/Game/UI/WB_HUD.WB_RoundStaminaBar` (`/Game/ThirdPerson/Blueprints/BP_ThirdPersonCharacter.HUD Widget` (`self.Player Character BP`))) (/ (`self.Current Stamina`) (`self.Max Stamina`))))

(fn `Increase Stamina`
  (params (`Added Stamina` :type "Float (double-precision)"))
  (set `self.Current Stamina` (+ (`self.Current Stamina`) `Added Stamina`))
  (if (> (`self.Current Stamina`) (`self.Max Stamina`))
    (set `self.Current Stamina` (`self.Max Stamina`)))
  (`/Game/UI/WB_RoundStaminaBar.SetPercentage` (`/Game/UI/WB_HUD.WB_RoundStaminaBar` (`/Game/ThirdPerson/Blueprints/BP_ThirdPersonCharacter.HUD Widget` (`self.Player Character BP`))) (/ (`self.Current Stamina`) (`self.Max Stamina`))))

(fn `Increase XP`
  (params (`Added XP` :type "Float (double-precision)"))
  (set `self.XP` (+ (`self.XP`) `Added XP`))
  (if (>= (`self.XP`) (`self.Max Xp`))
    (`self.Increase LVL` 1))
  (`ProgressBar.SetPercent` (`/Game/UI/WB_HUD.XPBar` (`/Game/ThirdPerson/Blueprints/BP_ThirdPersonCharacter.HUD Widget` (`self.Player Character BP`))) (/ (`self.XP`) (`self.Max Xp`)))
  (`TextBlock.SetText` (`/Game/UI/WB_HUD.XPText` (`/Game/ThirdPerson/Blueprints/BP_ThirdPersonCharacter.HUD Widget` (`self.Player Character BP`))) (`|FormatText` "{Current XP} / {Max XP}" (`self.XP`) (`self.Max Xp`))))
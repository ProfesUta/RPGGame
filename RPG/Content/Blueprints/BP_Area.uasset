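; BP_Area is an area marker that announces its name on screen when an actor tagged Player enters its trigger.
; The overlap creates a WB_MessagePopUp widget and plays its message animation with "Entering" followed by the AreaName variable.
; A DoOnce blocks repeat popups until a short delay ends, after which the widget is removed and the gate resets.
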(event `self.Trigger.OnComponentBeginOverlap`
  (params (OverlappedComponent :type "PrimitiveComponent Object Reference") (OtherActor :type "Actor Object Reference") (OtherComp :type "PrimitiveComponent Object Reference") (OtherBodyIndex :type Integer) (bFromSweep :type Boolean) (SweepResult :type "HitResult Structure (by ref)"))
  (if (`self.ActorHasTag` OtherActor "Player")
    (`/Engine/EditorBlueprintResources/StandardMacros.DoOnce` false :!label _label
      (:`Completed`
        (bind _returnvalue (`|CreateWidget` "/Game/UI/WB_MessagePopUp.WB_MessagePopUp_C"))
        (`UserWidget.AddToViewport` _returnvalue 0)
        (`/Game/UI/WB_MessagePopUp.PlayMessageAnimation` _returnvalue (`KismetTextLibrary.Conv_TextToString` (`|FormatText` "Entering {Area Name}" (`self.AreaName`))))
        (`KismetSystemLibrary.Delay` 0.1)
        (`KismetSystemLibrary.Delay` 3.25)
        (`/Engine/EditorBlueprintResources/StandardMacros.IsValid` _returnvalue
          (:`Is Valid`
            (`Widget.RemoveFromParent` _returnvalue)
            (goto _label :!via `Reset`))
          (:`Is Not Valid`
            (goto _label :!via `Reset`)))))))

(fn `UserConstructionScript`)
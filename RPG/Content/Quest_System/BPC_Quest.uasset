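; BPC_Quest is a quest component that shows the active quest on a HUD widget.
; On BeginPlay it creates a WB_QuestHUD, stores the reference and adds it to the viewport.
; Separate events push the ActiveQuest name into the HUD text and pass its objectives to the widget's FillObjectives function.
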(event `self.ReceiveBeginPlay`
  (bind _returnvalue (`|CreateWidget` "/Game/Quest_System/WB_QuestHUD.WB_QuestHUD_C"))
  (bind _output_get (set `self.QuestHudWidget` _returnvalue))
  (`UserWidget.AddToViewport` _output_get 0))

(event `Set Active Quest Text`
  (`TextBlock.SetText` (`/Game/Quest_System/WB_QuestHUD.ActiveQuestText` (`self.QuestHudWidget`)) (`KismetTextLibrary.Conv_StringToText` (`.Name_3_889894014B17F1EC9DEB34ABA2041162` (break `/Game/Quest_System/S_Quest` (`self.ActiveQuest`))))))

(event `SetObjectives`
  (bind (_activequest_name _activequest_description _activequest_secondary _activequest_complated _activequest_objectives) (break `/Game/Quest_System/S_Quest` (`self.ActiveQuest`)))
  (`/Game/Quest_System/WB_QuestHUD.Fill Objectives` (`self.QuestHudWidget`) _activequest_objectives))